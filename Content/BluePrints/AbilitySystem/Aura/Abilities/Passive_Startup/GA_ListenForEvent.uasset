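; Passive startup Gameplay Ability for Aura that listens for gameplay events under the Attributes tag and turns them into gameplay effects on its owner.
; Each event builds a spec from EventBasedEffectClass and compares the event tag against the EventTags array.
; A match passes the event magnitude as SetByCaller under that tag, while non-matches assign zero with no tag specified.
; The finished spec is then applied to self.
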(event Ability|EventActivateAbility
  (bind _returnvalue (Ability|GetAbilitySystemComponentfromActorInfo))
  (Development|PrintString "Listen for Event Activated" true true "(R=0.000000,G=0.290325,B=1.000000,A=1.000000)")
  (bind _payload (Ability|Tasks|WaitGameplayEvent "(TagName=\"Attributes\")" 0 false false)
    (:EventReceived
      (Variables|Default|SetEvent%20Tag (.EventTag (Utilities|Struct|BreakGameplayEventData _payload)))
      (Variables|Default|SetEvent%20Magnitude (.EventMagnitude (Utilities|Struct|BreakGameplayEventData _payload)))
      (Variables|Default|SetSpec (GameplayEffects|MakeOutgoingSpec _returnvalue (Variables|Default|GetEventBasedEffectClass) 1.0 (GameplayEffects|MakeEffectContext _returnvalue)))
      (for _array_element (Variables|Default|GetEventTags)
        (if (GameplayTags|MatchesTag _array_element (Variables|Default|GetEvent%20Tag))
          (Ability|GameplayEffect|AssignTagSetbyCallerMagnitude (Variables|Default|GetSpec) (Variables|Default|GetEvent%20Tag) (Variables|Default|GetEvent%20Magnitude))
          (else
            (Ability|GameplayEffect|AssignTagSetbyCallerMagnitude :SpecHandle (Variables|Default|GetSpec)))))
      (GameplayEffects|ApplyGameplayEffectSpecToSelf (Ability|GetAbilitySystemComponentfromActorInfo) (Variables|Default|GetSpec)))))